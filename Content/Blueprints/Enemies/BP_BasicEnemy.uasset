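; BP_BasicEnemy is a simple enemy that chases the player hero and dies after enough projectile hits.
; Every Tick it issues an AI MoveTo toward the player's BP_HeroCharacter.
; Overlapping a BP_Projectile calls a custom TakeDamage event, which removes one Life and destroys the actor when Life drops below one, and also prints the projectile's name.
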(event `self.ReceiveActorBeginOverlap`
  (params (OtherActor :type "Actor Object Reference"))
  (bind _asbp_projectile (cast `/Game/Blueprints/Weapons/BP_Projectile` OtherActor))
  (`self.TakeDamage`)
  (`KismetSystemLibrary.PrintString` (`KismetSystemLibrary.GetObjectName` _asbp_projectile)))

(event `self.ReceiveTick`
  (params (DeltaSeconds :type "Float (single-precision)"))
  ;[1 1 1] Move to Target
  (bind _asbp_hero_character (cast `/Game/Blueprints/Player/BP_HeroCharacter` (`GameplayStatics.GetPlayerCharacter` 0)))
  (`|AIMoveTo` self (0.0 0.0 0.0) _asbp_hero_character))

(event `TakeDamage`
  ;[1 1 1] Life
  (bind _output_get (set `self.Life` (- (`self.Life`) 1)))
  (if (< _output_get 1)
    (`self.K2_DestroyActor`)))

(fn `UserConstructionScript`)