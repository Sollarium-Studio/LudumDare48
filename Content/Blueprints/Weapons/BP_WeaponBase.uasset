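; Base weapon Blueprint that handles automatic projectile fire, magazine ammo and reloading.
; FireEvent shoots immediately, then loops WeaponFire on a timer set by ShootPerSecond, spawning BP_Projectile at the Muzzle socket until StopFireEvent clears it.
; An empty magazine or ReloadEvent pauses firing and starts a timed ReloadWeapon call, which refills bullets and resumes fire if IsFiring is still set.
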(event `FireEvent`
  ;[1 1 1] Fire and stop fire event
  (set `self.IsFiring` true)
  (`self.WeaponFire`)
  (`KismetSystemLibrary.K2_SetTimer` null "WeaponFire" (/ 1.0 (`self.ShootPerSecond`)) true))

(event `StopFireEvent`
  ;[1 1 1] Fire and stop fire event
  (`KismetSystemLibrary.K2_ClearTimer` null "WeaponFire")
  (set `self.IsFiring` false))

(event `ReloadEvent`
  ;[1 1 1] Reload
  (set `self.Reloading` true)
  (`KismetSystemLibrary.K2_SetTimer` null "ReloadWeapon" 1.0)
  (`KismetSystemLibrary.K2_ClearTimer` null "WeaponFire")
  (`KismetSystemLibrary.PrintString` "Reloading..."))

(fn `ReloadWeapon`
  (set `self.CurrentBullets` (`self.TotalAmmoInAmmo`))
  (set `self.Reloading` false)
  (`KismetSystemLibrary.PrintString` "Reloaded")
  (if (`self.IsFiring`)
    (`self.WeaponFire`)
    (`KismetSystemLibrary.K2_SetTimer` null "WeaponFire" (/ 1.0 (`self.ShootPerSecond`)) true)))

(fn `UserConstructionScript`)

(fn `WeaponFire`
  (if (> (`self.CurrentBullets`) 0)
    (if (not (`self.Reloading`))
      (`|SpawnActorFromClass` "/Game/Blueprints/Weapons/BP_Projectile.BP_Projectile_C" (`SceneComponent.GetSocketTransform` (`self.WeaponSketetalMesh`) "Muzzle" "RTS_World") "AlwaysSpawn" "OverrideRootScale" null null)
      (set `self.CurrentBullets` (- (`self.CurrentBullets`) 1)))
    (elif (not (`self.Reloading`))
      (`KismetSystemLibrary.K2_SetTimer` null "ReloadWeapon" 1.0)
      (`KismetSystemLibrary.K2_ClearTimer` null "WeaponFire")
      (set `self.Reloading` true)
      (`KismetSystemLibrary.PrintString` "Reloading..."))))